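; BP_CharCtrl is a controller that moves its pawn toward the mouse cursor while the Mouse input action is held.
; Press and release set a flag that Tick checks each frame.
; While set, Tick traces under the cursor on the Visibility channel and feeds the direction from pawn to hit location into AddMovementInput.
; Movement is direct steering, with no pathfinding or check that the trace hit.
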(event EventBeginPlay)

(event EventTick
  (params (DeltaSeconds :type Float%20%28single-precision%29))
  (bind _returnvalue (Pawn|GetControlledPawn))
  (if (Variables|Default|GetmMouseClick)
    (Pawn|Input|AddMovementInput _returnvalue (Math|Vector|GetUnitDirection(Vector) (Transformation|GetActorLocation _returnvalue) (.Location (Collision|BreakHitResult (.HitResult (Game|Player|GetHitResultUnderCursorbyChannel "TraceTypeQuery1" true))))) 1.0 false)))

(event Input|ActionEvents|InputActionMouse
  (params (Key :type Key%20Structure))
  (:Pressed
    (Variables|Default|SetmMouseClick true))
  (:Released
    (Variables|Default|SetmMouseClick false)))

(fn ConstructionScript)